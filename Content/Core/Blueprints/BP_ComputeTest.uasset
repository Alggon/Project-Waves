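; BP_ComputeTest is a test actor that floats a physics cube on waves from the WaveComputeSubsystem.
; Five scene components act as floater points, gathered into an array at BeginPlay.
; Each tick, every floater below the sampled wave height pushes the cube up at its location, scaled by depth and FloatingPower and divided by floater count.
; A constant push and debug sphere drawing are left disconnected.
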(event `self.ReceiveBeginPlay`
  (set `self.Floaters` (`|MakeArray` (`self.Scene`) (`self.Scene1`) (`self.Scene2`) (`self.Scene3`) (`self.Scene4`))))

(event `self.ReceiveTick`
  (params (DeltaSeconds :type "Float (single-precision)"))
  ; It works
  (for _array_element (`self.Floaters`)
    (bind _returnvalue (`SceneComponent.K2_GetComponentLocation` _array_element))
    (bind _returnvalue_2 (- (.z _returnvalue) (.z (* (`WaveComputeSubsystem.GetWaveHeightAtWorldPos` (subsystem `WaveComputeSubsystem`) _returnvalue) (1.0 1.0 1.0)))))
    (if (< _returnvalue_2 0.0)
      (`PrimitiveComponent.AddForceAtLocation` (`self.Cube`) (/ (* (`KismetMathLibrary.Vector_Up`) (`KismetMathLibrary.Abs` _returnvalue_2) (`self.FloatingPower`)) (`KismetMathLibrary.Conv_IntToDouble` (`KismetArrayLibrary.Array_Length` (`self.Floaters`)))) _returnvalue "None"))))

(fn `UserConstructionScript`)